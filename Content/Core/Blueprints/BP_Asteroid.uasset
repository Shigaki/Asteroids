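; BP_Asteroid is an asteroid actor that hurts the player on contact and takes damage itself in return.
; When a living BP_PlayerCharacter overlaps its mesh, a DoOnce applies damage to the player and heavier damage to the asteroid, crediting the player as instigator.
; Random mesh selection from DT_Asteroids is present but disconnected, so the construction script does nothing.
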(event `self.Mesh.OnComponentBeginOverlap`
  (params (OverlappedComponent :type "PrimitiveComponent Object Reference") (OtherActor :type "Actor Object Reference") (OtherComp :type "PrimitiveComponent Object Reference") (OtherBodyIndex :type Integer) (bFromSweep :type Boolean) (SweepResult :type "HitResult Structure (by ref)"))
  (bind _asbp_player_character (cast `/Game/Core/Player/BP_PlayerCharacter` OtherActor))
  (bind _returnvalue (`AsteroidsPlayerCharacter.IsDead` _asbp_player_character))
  (if (not _returnvalue)
    (`/Engine/EditorBlueprintResources/StandardMacros.DoOnce` false
      (:`Completed`
        (`GameplayStatics.ApplyDamage` _asbp_player_character 1.0 null self)
        (`GameplayStatics.ApplyDamage` self 10.0 (`self.GetInstigatorController` _asbp_player_character) _asbp_player_character)))))

(fn `UserConstructionScript`)