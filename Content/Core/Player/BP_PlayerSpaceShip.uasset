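; Player spaceship Blueprint for multiplayer, with randomized colors and projectile firing.
; On BeginPlay the authority picks random hull and turbine colors, and their RepNotify functions apply them through dynamic material instances on the ship mesh.
; Fire input goes to the multicast event, via a server RPC from clients, so each machine spawns its own projectile at the fire location, rate-limited by a DoOnce and Delay cooldown.
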(event `self.ReceiveBeginPlay`
  (`/Engine/EditorBlueprintResources/ActorMacros.Switch Has Authority`
    (:`Authority`
      (set `self.OsnColor` (make `LinearColor` (`KismetMathLibrary.RandomFloat`) (`KismetMathLibrary.RandomFloat`) (`KismetMathLibrary.RandomFloat`) 1.0))
      (set `self.TurbineColor` (make `LinearColor` (`KismetMathLibrary.RandomFloat`) (`KismetMathLibrary.RandomFloat`) (`KismetMathLibrary.RandomFloat`) 1.0)))))

(event `InputAction|FireProjectile`
  (params (Key :type "Key Structure"))
  (:`Pressed`
    (`/Engine/EditorBlueprintResources/ActorMacros.Switch Has Authority`
      (:`Authority`
        (`self.MC_FireProjectile`))
      (:`Remote`
        (`self.Server_FireProjectile`)))))

(event `MC_FireProjectile`
  (`/Engine/EditorBlueprintResources/StandardMacros.DoOnce` false :!label _label
    (:`Completed`
      (`|SpawnActorFromClass` "/Game/Core/Blueprints/BP_Projectile.BP_Projectile_C" (`KismetMathLibrary.MakeTransform` (`SceneComponent.K2_GetComponentLocation` (`self.FireLocation`)) (`self.K2_GetActorRotation`)) "AlwaysSpawn" "OverrideRootScale" self (`self.Instigator`))
      (`KismetSystemLibrary.Delay` 0.2)
      (goto _label :!via `Reset`))))

(event `Server_FireProjectile`
  (`self.MC_FireProjectile`))

(fn `OnRep_OsnColor`
  (bind _returnvalue (`PrimitiveComponent.CreateDynamicMaterialInstance` (`self.SM_Spaceship`) 0 "/Game/Imports/SpaceshipUnitron/MI_Osn.MI_Osn" "None"))
  (`MaterialInstanceDynamic.SetVectorParameterValue` _returnvalue "BaseColor" (`self.OsnColor`)))

(fn `OnRep_TurbineColor`
  (bind _returnvalue (`PrimitiveComponent.CreateDynamicMaterialInstance` (`self.SM_Spaceship`) 1 "/Game/Imports/SpaceshipUnitron/MI_Turbine.MI_Turbine" "None"))
  (`MaterialInstanceDynamic.SetVectorParameterValue` _returnvalue "BaseColor" (`self.TurbineColor`)))

(fn `UserConstructionScript`)