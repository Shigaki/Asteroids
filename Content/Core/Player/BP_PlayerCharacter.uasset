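; Player spaceship character with randomized colors and a proximity-based revive when dead.
; The authority rolls two colors at BeginPlay, and their RepNotifies apply them through dynamic material instances on the hull and turbine slots.
; While dead, overlap by a Player-tagged actor starts a looping timer that fills a widget progress bar; ending overlap hides it and cancels.
; A full bar hides the widget, and only the authority calls Ressurect.
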(event `self.ReceiveBeginPlay`
  (`/Engine/EditorBlueprintResources/ActorMacros.Switch Has Authority`
    (:`Authority`
      (set `self.OsnColor` (make `LinearColor` (`KismetMathLibrary.RandomFloat`) (`KismetMathLibrary.RandomFloat`) (`KismetMathLibrary.RandomFloat`) 1.0))
      (set `self.TurbineColor` (make `LinearColor` (`KismetMathLibrary.RandomFloat`) (`KismetMathLibrary.RandomFloat`) (`KismetMathLibrary.RandomFloat`) 1.0)))))

(event `self.SpaceshipMesh.OnComponentBeginOverlap`
  (params (OverlappedComponent :type "PrimitiveComponent Object Reference") (OtherActor :type "Actor Object Reference") (OtherComp :type "PrimitiveComponent Object Reference") (OtherBodyIndex :type Integer) (bFromSweep :type Boolean) (SweepResult :type "HitResult Structure (by ref)"))
  (bind _pbwidget (`self.PBWidget`))
  (bind _returnvalue (`self.IsDead`))
  (if (and _returnvalue (`self.ActorHasTag` OtherActor "Player"))
    (bind _aswbp_progress_bar (cast `/Game/Core/UI/WBP_ProgressBar` (`WidgetComponent.GetWidget` _pbwidget)))
    (set `/Game/Core/UI/WBP_ProgressBar.ProgressBarValue` 0.0 _aswbp_progress_bar)
    (`SceneComponent.SetHiddenInGame` _pbwidget false false)
    (bind _returnvalue_2 (`KismetSystemLibrary.K2_SetTimer` null "FillProgressBar" 0.02 true))
    (set `self.ProgresBarHandler` _returnvalue_2)))

(event `self.SpaceshipMesh.OnComponentEndOverlap`
  (params (OverlappedComponent :type "PrimitiveComponent Object Reference") (OtherActor :type "Actor Object Reference") (OtherComp :type "PrimitiveComponent Object Reference") (OtherBodyIndex :type Integer))
  (bind _returnvalue (`self.IsDead`))
  (if (and _returnvalue (`self.ActorHasTag` OtherActor "Player"))
    (`SceneComponent.SetHiddenInGame` (`self.PBWidget`) true false)
    (`KismetSystemLibrary.K2_ClearAndInvalidateTimerHandle` (`self.ProgresBarHandler`))))

(fn `FillProgressBar`
  (bind _aswbp_progress_bar (cast `/Game/Core/UI/WBP_ProgressBar` (`WidgetComponent.GetWidget` (`self.PBWidget`))))
  (bind _output_get (set `/Game/Core/UI/WBP_ProgressBar.ProgressBarValue` (+ (`/Game/Core/UI/WBP_ProgressBar.ProgressBarValue` _aswbp_progress_bar) 0.01) _aswbp_progress_bar))
  (if (>= _output_get 1.0)
    (`SceneComponent.SetHiddenInGame` (`self.PBWidget`) true false)
    (`KismetSystemLibrary.K2_ClearAndInvalidateTimerHandle` (`self.ProgresBarHandler`))
    (`/Engine/EditorBlueprintResources/ActorMacros.Switch Has Authority`
      (:`Authority`
        (`self.Ressurect`)))))

(fn `OnRep_OsnColor`
  (bind _returnvalue (`PrimitiveComponent.CreateDynamicMaterialInstance` (`self.SpaceshipMesh`) 0 "/Game/Imports/SpaceshipUnitron/MI_Osn.MI_Osn" "None"))
  (`MaterialInstanceDynamic.SetVectorParameterValue` _returnvalue "BaseColor" (`self.OsnColor`)))

(fn `OnRep_TurbineColor`
  (bind _returnvalue (`PrimitiveComponent.CreateDynamicMaterialInstance` (`self.SpaceshipMesh`) 1 "/Game/Imports/SpaceshipUnitron/MI_Turbine.MI_Turbine" "None"))
  (`MaterialInstanceDynamic.SetVectorParameterValue` _returnvalue "BaseColor" (`self.TurbineColor`)))

(fn `UserConstructionScript`)